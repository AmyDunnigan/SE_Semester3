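; BP_TestDamageWall4 is a functional test that checks a character walking into a BP_DamageWall triggers its hit event.
; On test start it binds WallHit to the OnHitWall event of every damage wall in the level.
; Each tick it forces the character to a fixed rotation and feeds forward movement input.
; A true hit state finishes the test as succeeded, with no explicit failure path.
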(event Custom|WallHit
  (params (HitState :type Boolean))
  (if HitState
    (Class|FunctionalTest|FinishTest "Succeeded" "Test succeeded!")))

(event EventPrepareTest)

(event EventStartTest
  (bind _outactors (Actor|GetAllActorsOfClass "/Game/BP_DamageWall.BP_DamageWall_C"))
  (for _array_element _outactors
    (EventDispatchers|BindEventtoOnHitWall _array_element (delegate Custom|WallHit))))

(event EventTick
  (params (DeltaSeconds :type Float%20%28single-precision%29))
  (bind _character (Variables|Default|GetCharacter))
  (Transformation|SetActorRotation (Variables|Default|GetCharacter) "0.000000,270.000000,0.000000")
  (Pawn|Input|AddMovementInput _character (Transformation|GetActorForwardVector _character) 1.0 false))

(fn ConstructionScript)