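; Functional test that checks the player controller's SetSpawnRange call spawns one falling rock.
; On test start it counts BP_FallingRock actors, calls SetSpawnRange on player 0's MyPlayerController, then asserts the count rose by exactly one.
; It finishes as succeeded only when the assertion passes; a failed cast or assertion never calls FinishTest.
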(event EventPrepareTest)

(event EventStartTest
  (bind _outactors (Actor|GetAllActorsOfClass "/Game/BP_FallingRock.BP_FallingRock_C"))
  (Variables|Default|SetPreSpawnActors (Utilities|Array|Length _outactors))
  (bind _asmy_player_controller (Utilities|Casting|CastToMyPlayerController (Game|GetPlayerController 0)))
  (Default|SetSpawnRange _asmy_player_controller)
  (bind _outactors_2 (Actor|GetAllActorsOfClass "/Game/BP_FallingRock.BP_FallingRock_C"))
  (bind _returnvalue (Class|FunctionalTest|AssertEqualInt (Utilities|Array|Length _outactors_2) (+ (Variables|Default|GetPreSpawnActors) 1)))
  (if _returnvalue
    (Class|FunctionalTest|FinishTest "Succeeded" "Rocks are spawning")))

(event EventTick
  (params (DeltaSeconds :type Float%20%28single-precision%29)))

(fn ConstructionScript)