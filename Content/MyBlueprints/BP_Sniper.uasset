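; BP_Sniper is a hazard actor that strikes actors entering its overlap area after a short delay.
; One timer launches player character 0, and a looping timer repeatedly damages the overlapping actor, both firing sniper-strike notifications.
; End overlap clears only the damage timer, because its handle overwrites the launch handle.
; The Player-tag check is not wired into the overlap flow, and DecreaseHealthIncrement is empty.
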(event Custom|ApplyDamage
  (Game|Damage|ApplyDamage (stale Collision|EventActorBeginOverlap OtherActor) 1e+02 0 0)
  (Default|CallOnSniperStrike true))

(event Custom|LaunchEvent
  (CallFunction|LaunchPlayer (stale Collision|EventActorBeginOverlap OtherActor))
  (Default|CallOnSniperStrike true))

(event Collision|EventActorEndOverlap
  (params (OtherActor :type Actor%20Object%20Reference))
  (Utilities|Time|ClearandInvalidateTimerbyHandle (Variables|Default|GetTimerReference)))

(event Collision|EventActorBeginOverlap
  (params (OtherActor :type Actor%20Object%20Reference))
  (Utilities|IsValid OtherActor
    (:Is%20Valid
      (Utilities|FlowControl|Delay 2.0)
      (bind _returnvalue (Utilities|Time|SetTimerbyEvent (delegate Custom|LaunchEvent) 0.05))
      (Variables|Default|SetTimerReference _returnvalue)
      (bind _returnvalue_2 (Utilities|Time|SetTimerbyEvent (delegate Custom|ApplyDamage) 0.06 true))
      (Variables|Default|SetTimerReference _returnvalue_2))))

(fn ConstructionScript)

(fn LaunchPlayer
  (params (self2 :type Actor%20Object%20Reference))
  (Character|LaunchCharacter (Game|GetPlayerCharacter 0) (- (Transformation|GetActorForwardVector self2) "500.000000,500.000000,-50.000000") true true)
  (Default|CallOnLaunchPlayer true))

(fn HasPlayerTag
  (params (self2 :type Actor%20Object%20Reference))
  (if (Actor|ActorHasTag self2 "Player")
    (Default|CallOnPlayerTagged true)))

(fn DecreaseHealthIncrement)