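; BP_DamageWall is an actor that deals periodic damage to a Player-tagged actor while it overlaps the wall.
; Begin overlap starts a looping one-second timer that applies fixed damage to that actor and fires the OnHitWall dispatcher on each tick.
; End overlap clears the stored timer without checking the tag, so any actor leaving stops the damage.
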(event Custom|ApplyDamage
  (Game|Damage|ApplyDamage (stale Collision|EventActorBeginOverlap OtherActor) 1e+01 0 0)
  (Default|CallOnHitWall true))

(event EventBeginPlay)

(event Collision|EventActorEndOverlap
  (params (OtherActor :type Actor%20Object%20Reference))
  (Utilities|Time|ClearandInvalidateTimerbyHandle (Variables|Default|GetTimerReference)))

(event EventTick
  (params (DeltaSeconds :type Float%20%28single-precision%29)))

(event Collision|EventActorBeginOverlap
  (params (OtherActor :type Actor%20Object%20Reference))
  (if (Actor|ActorHasTag OtherActor "Player")
    (bind _returnvalue (Utilities|Time|SetTimerbyEvent (delegate Custom|ApplyDamage) 1.0 true))
    (Variables|Default|SetTimerReference _returnvalue)))

(fn ConstructionScript)